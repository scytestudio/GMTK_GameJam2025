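; BP_KeyBoard is a keyboard actor that shows idle or playing Paper2D flipbook animations on separate left and right halves.
; UpdateKeyboardState stores the new state and sets both flipbooks for Idle, Play Left or Play Both, and BeginPlay starts it in Play Left.
; A right-only playing combination exists in the graph but is unconnected, so it never runs.
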(event `self.ReceiveBeginPlay`
  (`self.UpdateKeyboardState` "EKS_PlayLeft"))

(event `UpdateKeyboardState`
  (params (NewState :type "EGMTK_KeyboardStates Enum" :default "EKS_Idle"))
  (bind _leftplayflbk (`self.LeftPlayFLBK`))
  (bind _leftkeyboard (`self.LeftKeyboard`))
  (bind _rightidleflbk (`self.RightIdleFLBK`))
  (bind _rightkeyboard (`self.RightKeyboard`))
  (bind _output_get (set `self.KeyboardState` NewState))
  (switch `EGMTK_KeyboardStates` _output_get
    (:`EKS_Idle`
      (`PaperFlipbookComponent.SetFlipbook` _leftkeyboard (`self.LeftIdleFLBK`))
      (`PaperFlipbookComponent.SetFlipbook` _rightkeyboard _rightidleflbk))
    (:`EKS_PlayLeft`
      (`PaperFlipbookComponent.SetFlipbook` _leftkeyboard _leftplayflbk)
      (`PaperFlipbookComponent.SetFlipbook` _rightkeyboard _rightidleflbk))
    (:`EKS_PlayBoth`
      (`PaperFlipbookComponent.SetFlipbook` _leftkeyboard _leftplayflbk)
      (`PaperFlipbookComponent.SetFlipbook` _rightkeyboard (`self.RightPlayFLBK`)))))

(fn `UserConstructionScript`)