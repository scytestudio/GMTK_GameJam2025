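; BP_CatBase is a base side-scrolling sprite cat character with move, jump and forward dash events, all gated by CanMove.
; Movement runs along world X and flips the sprite by negative scale, tracking FacingRight and enabling CanDash for nonzero input.
; The grounded-only dash launches the cat up and forward, plays an animation override, then re-enables CanDash after its duration, though movement input can re-enable it sooner.
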(event `self.ReceiveBeginPlay`)

(event `MoveCat`
  (params (ScaleValue :type "Float (double-precision)"))
  (if (`self.bCanMove`)
    (`self.UpdateDirection` ScaleValue)
    (`self.AddMovementInput` (1.0 0.0 0.0) ScaleValue)))

(event `JumpCat`
  (if (`self.bCanMove`)
    (`self.Jump`)))

(event `UpdateDirection`
  (params (Direction :type "Float (double-precision)"))
  ;[1 1 1] Update Direction Logic
  (if (< Direction 0.0)
    (`SceneComponent.SetWorldScale3D` (`self.Sprite`) (-0.25 0.25 0.25))
    (set `self.bFacingRight?` false)
    (set `self.bCanDash` true :!label _label)
    (elif (> Direction 0.0)
      (`SceneComponent.SetWorldScale3D` (`self.Sprite`) (0.25 0.25 0.25))
      (set `self.bFacingRight?` true)
      (goto _label)
      (else
        (set `self.bCanDash` false)))))

(event `DashForward`
  (if (and (`self.bCanDash`) (`self.bCanMove`) (not (`NavMovementComponent.IsFalling` (`self.CharacterMovement`))))
    (set `self.bCanDash` false)
    (`self.LaunchCharacter` (`KismetMathLibrary.MakeVector` (`KismetMathLibrary.SelectFloat` 1000.0 -1000.0 (`self.bFacingRight?`)) 0.0 1000.0))
    (bind _animationlength (`PaperZDAnimInstance.K2_PlayAnimationOverride` (`self.GetAnimInstance`) "/Game/Core/Blueprints/Characters/Cat/Animation/AnimSequences/CatDash.CatDash" "DefaultSlot" 1.0 0.0))
    (`KismetSystemLibrary.Delay` _animationlength)
    (set `self.bCanDash` true)))

(fn `UserConstructionScript`)