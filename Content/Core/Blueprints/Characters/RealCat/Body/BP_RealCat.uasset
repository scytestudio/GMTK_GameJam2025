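; BP_RealCat is the cat body, switching animation states on a timer and driving the separate BP_RealCatHand actor found at BeginPlay.
; A looping timer, its interval randomized once, checks CurrentState, which this graph never sets, and sends animation messages: Petting leads to Sleep, Sleep to Awake.
; It also writes the hand's state directly: idle after Petting, alternating moving and idle through a FlipFlop after Sleep.
; An unconnected Petting branch never runs.
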(event `self.ReceiveBeginPlay`
  (bind _returnvalue (`GameplayStatics.GetActorOfClass` "/Game/Core/Blueprints/Characters/RealCat/Hand/BP_RealCatHand.BP_RealCatHand_C"))
  (set `self.CatHandRef` _returnvalue)
  (`KismetSystemLibrary.K2_SetTimerDelegate` (delegate `UpdateCatBody`) (`KismetMathLibrary.RandomFloatInRange` 5.0 10.0) true))

(event `UpdateCatBody`
  (switch `EGMTK_RealCatBodyStates` (`self.CurrentState`)
    (:`ERCS_Petting`
      (message `RealCatInterface.UpdateCatBodyAnimation` self "ERCS_Sleep")
      (`self.UpdateCatHand` "ERCS_HandIdle"))
    (:`ERCS_Sleep`
      (message `RealCatInterface.UpdateCatBodyAnimation` self "ERCS_Awake")
      (`/Engine/EditorBlueprintResources/StandardMacros.FlipFlop`
        (:`A`
          (`self.UpdateCatHand` "ERCS_HandMoving"))
        (:`B`
          (`self.UpdateCatHand` "ERCS_HandIdle"))))))

(event `UpdateCatHand`
  (params (CurrentHandState :type "EGMTK_RealCatHandStates Enum" :default "ERCS_HandIdle"))
  (set `/Game/Core/Blueprints/Characters/RealCat/Hand/BP_RealCatHand.CurrentHandState` CurrentHandState (`self.CatHandRef`)))

(fn `UserConstructionScript`)