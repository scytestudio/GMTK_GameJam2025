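; BP_MainCamera relays player input to the cat character, despite its camera name; its graphs contain no camera logic.
; On BeginPlay it caches the BP_CatBase actor found in the level and adds the IMC_CatMap Enhanced Input context to the PC_PlayerController.
; Move and jump input actions are forwarded to that cached cat after a validity check, with releasing jump calling StopJumping.
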(event `self.ReceiveBeginPlay`
  (bind _returnvalue (`GameplayStatics.GetActorOfClass` "/Game/Core/Blueprints/Characters/Cat/BP_CatBase.BP_CatBase_C"))
  (set `self.CatRef` _returnvalue)
  (bind _aspc_player_controller (cast `/Game/Core/Blueprints/Game/PC_PlayerController` (`GameplayStatics.GetPlayerController` 0)))
  (`EnhancedInputSubsystemInterface.AddMappingContext` (pcsubsystem `EnhancedInputLocalPlayerSubsystem` _aspc_player_controller) "/Game/Core/Inputs/IMC_CatMap.IMC_CatMap" 0 (struct)))

(event `EnhancedInput|/Game/Core/Inputs/Actions/IA_MoveCat`
  (params (ActionValue :type "Float (double-precision)") (ElapsedSeconds :type "Float (double-precision)") (TriggeredSeconds :type "Float (double-precision)") (InputAction :type "InputAction Object Reference" :default "/Game/Core/Inputs/Actions/IA_MoveCat.IA_MoveCat"))
  ;[0.1117 0.2492 1] CAT - Move Input
  (:`Triggered`
    (bind _catref (`self.CatRef`)
      (:`then`
        (`/Game/Core/Blueprints/Characters/Cat/BP_CatBase.MoveCat` _catref ActionValue))
      (:`else`))))

(event `EnhancedInput|/Game/Core/Inputs/Actions/IA_JumpCat`
  (params (ActionValue :type Boolean) (ElapsedSeconds :type "Float (double-precision)") (TriggeredSeconds :type "Float (double-precision)") (InputAction :type "InputAction Object Reference" :default "/Game/Core/Inputs/Actions/IA_JumpCat.IA_JumpCat"))
  ;[0.1117 0.2492 1] CAT ---- Jump Input
  (:`Started`
    (bind _catref (`self.CatRef`)
      (:`then`
        (`Character.Jump` _catref))
      (:`else`)))
  (:`Completed`
    (bind _catref_2 (`self.CatRef`)
      (:`then`
        (`Character.StopJumping` _catref_2))
      (:`else`))))

(fn `UserConstructionScript`)